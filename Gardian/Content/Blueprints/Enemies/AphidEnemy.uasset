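; Aphid enemy that crawls toward its guardian plant and, once within stopping range, runs a looping timer to damage it, with tuning read from the GameplayTuning data table.
; Tick drives straight-line movement on the horizontal plane until StopUpdate is set, which also clears the damage timer.
; DealDamage sets that flag, swaps to the Attack mesh, disables collision and starts a short timer, while a dynamic material supports flashing before particle-spawning death.
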(event Custom|Begin%20Death
  (Game|SpawnActorfromClass "/Game/Blueprints/deathParticles.deathParticles_C" (Transformation|GetActorTransform) "Undefined" 0 0)
  (Actor|DestroyActor))

(event EventBeginPlay
  (CallFunction|InitalizeDefaultsfromDataTable)
  ;[1 1 1] make new material
  (bind _returnvalue (Rendering|Material|CreateDynamicMaterialInstance "/Game/Materials/AphidBody.AphidBody" "None" :!class /Script/Engine.KismetMaterialLibrary))
  (bind _output_get (Variables|Default|Setmaterial _returnvalue))
  (Rendering|Material|SetMaterial (Variables|Default|GetSkeletalMesh) 0 _output_get)
  (Utilities|Time|SetTimerbyEvent (EventDispatchers|CreateEvent :!event Flash) 0.05 true))

(event Collision|EventActorBeginOverlap
  (params (OtherActor :type Actor%20Object%20Reference)))

(event EventTick
  (params (DeltaSeconds :type Float%20%28single-precision%29))
  (if (Variables|Default|GetStopUpdate!)
    (if (Utilities|Time|IsValidTimerHandle (Variables|Default|GetDamagePlantTimerHandle))
      (Utilities|Time|ClearandInvalidateTimerbyHandle (Variables|Default|GetDamagePlantTimerHandle))
      (Variables|Default|SetisDamageTimerON? false))
    (else
      (CallFunction|UpdateMovement DeltaSeconds))))

(fn ConstructionScript
  (|CallParentFunction))

(fn SetGardianPlant
  (params (TargetPlant :type Plant%20Object%20Reference))
  (Variables|Default|SetGardianPlant TargetPlant))

(fn GetDirectiontoPlant
  (bind _self self)
  (bind _gardianplant (Variables|Default|GetGardianPlant))
  (bind _returnvalue (Transformation|GetActorLocation _gardianplant))
  (bind _returnvalue_2 (Transformation|GetActorLocation _self))
  (bind _returnvalue_3 (- _returnvalue _returnvalue_2))
  (return (Math|Vector|Normalize (Math|Vector|MakeVector (.x _returnvalue_3) (.y _returnvalue_3) 0.0))))

(fn UpdateMovement
  (params (DeltaTime :type Float%20%28single-precision%29))
  (Utilities|FlowControl|Sequence
    (:then_0
      (bind _output_get (LocalVariables|SetMovedLocation (+ (* (CallFunction|GetDirectiontoPlant) (* DeltaTime (Variables|Default|GetSpeed))) (Transformation|GetActorLocation)))) ; Get distance from plant
      (LocalVariables|SetdistanceFromPlant (Math|Vector|VectorLength (- _output_get (Transformation|GetActorLocation (Variables|Default|GetGardianPlant))))))
    (:then_1
      (if (> (LocalVariables|GetdistanceFromPlant) (Variables|Default|GetStopAtDistance))
        (Transformation|SetActorLocation (LocalVariables|GetMovedLocation) false false)
        (else
          (Utilities|FlowControl|Sequence ; Reached to the Plant
            (:then_0
              (Audio|Components|Audio|Stop (Variables|Default|GetSkeletalMesh)))
            (:then_1
              (if (not (Variables|Default|GetisDamageTimerON?))
                (bind _returnvalue (Utilities|Time|SetTimerbyEvent (EventDispatchers|CreateEvent :!event DamageGardianPlant) (Variables|Default|GetDealDamageEvery?Seconds) true))
                (Variables|Default|SetisDamageTimerON? true)
                (Variables|Default|SetDamagePlantTimerHandle _returnvalue)))))))))

(fn DealDamage
  (bind _skeletalmesh (Variables|Default|GetSkeletalMesh))
  (|CallParentFunction)
  (Class|SkinnedMeshComponent|SetSkeletalMesh _skeletalmesh "/Game/Animation/Aphid/Attack/Attack.Attack" true)
  (Components|Animation|SetAnimationMode _skeletalmesh "AnimationSingleNode")
  (Transformation|SetRelativeLocation (Variables|Default|GetSkeletalMesh) "-51.000000, 0, 0" false true)
  (Variables|Default|SetStopUpdate! true)
  (Collision|SetCollisionEnabled (Variables|Default|GetStaticMesh) "NoCollision")
  (Collision|SetCollisionEnabled (Variables|Default|GetSkeletalMesh) "NoCollision")
  (Utilities|Time|SetTimerbyEvent (EventDispatchers|CreateEvent :!event Custom|Begin%20Death) 1.0))

(fn DamageGardianPlant
  (Default|Shrink (Variables|Default|GetGardianPlant) false))

(fn InitalizeDefaultsfromDataTable
  (Utilities|FlowControl|Sequence
    (:then_0
      (bind _returnvalue (Utilities|GetDataTableRow "/Game/DataTables/GameplayTuning.GameplayTuning" "AphidSpeed")
        (:then
          (Variables|Default|SetSpeed (.value _returnvalue)))))
    (:then_1
      (bind _returnvalue_2 (Utilities|GetDataTableRow "/Game/DataTables/GameplayTuning.GameplayTuning" "AphidStopAtDistance")
        (:then
          (Variables|Default|SetStopAtDistance (.value _returnvalue_2)))))
    (:then_2
      (bind _returnvalue_3 (Utilities|GetDataTableRow "/Game/DataTables/GameplayTuning.GameplayTuning" "AphidDealDamageToPlantTimer")
        (:then
          (Variables|Default|SetDealDamageEvery?Seconds (.value _returnvalue_3)))))))

(fn Flash
  (if (Variables|Default|GetStopUpdate!)
    (Variables|Default|SetflashState (not (Variables|Default|GetflashState)))
    (Rendering|Material|SetScalarParameterValue (Variables|Default|Getmaterial) "flash" (Math|Conversions|ToFloat(Boolean) (Variables|Default|GetflashState)) :!class /Script/Engine.MaterialInstanceDynamic)))