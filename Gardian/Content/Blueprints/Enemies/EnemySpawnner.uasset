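; Spawner actor that periodically creates aphid and weed enemies and hands each a reference to the guardian plant.
; On BeginPlay it reads spawn intervals and the weed cap from the GameplayTuning data table, then starts two looping timers unless disabled.
; Aphids spawn at random points in bug volumes, yawed toward the plant.
; Weeds spawn at random preset locations, filtering out occupied spots and respecting the cap.
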(event EventBeginPlay
  (CallFunction|InitializeDefaultsfromDataTable)
  (if (not (Variables|Default|GetDisabled))
    (Utilities|Time|SetTimerbyEvent (EventDispatchers|CreateEvent :!event SpawnNewBug) (Variables|Default|GetBug%20Spawn%20Timer) true)
    (Utilities|Time|SetTimerbyEvent (EventDispatchers|CreateEvent :!event CheckSpawnNewWeed) (Variables|Default|GetWeed%20Spawn%20Timer) true)))

(event Collision|EventActorBeginOverlap
  (params (OtherActor :type Actor%20Object%20Reference)))

(event EventTick
  (params (DeltaSeconds :type Float%20%28single-precision%29)))

(fn ConstructionScript)

(fn SpawnNewBug
  (bind _bug_spawn_volumes (Variables|Default|GetBug%20Spawn%20Volumes))
  (bind _bug_spawn_volumes_2 (Variables|Default|GetBug%20Spawn%20Volumes))
  (bind _returnvalue (Utilities|Array|Length _bug_spawn_volumes))
  (bind _returnvalue_2 (- _returnvalue 1))
  (bind _returnvalue_3 (Math|Random|RandomIntegerinRange 0 _returnvalue_2))
  (bind _output (Utilities|Array|Get(acopy) _bug_spawn_volumes_2 _returnvalue_3))
  (bind (_origin _boxextent) (Collision|GetActorBounds _output false))
  (if (> (Utilities|Array|Length (Variables|Default|GetBug%20Spawn%20Volumes)) 0)
    (LocalVariables|SetVolume%20Name (Utilities|GetObjectName _output))
    (bind _position_out (CallFunction|GetRandomPositionfromVolume _origin _boxextent))
    (bind _returnvalue_4 (Game|SpawnActorfromClass "/Game/Blueprints/Enemies/AphidEnemy.AphidEnemy_C" (Math|Transform|MakeTransform _position_out (Math|Rotator|MakeRotfromX (* (Math|Vector|Normalize (Math|Vector|MakeVector (.x (- _position_out (Transformation|GetActorLocation (Variables|Default|GetGardian%20Plant)))) (.y (- _position_out (Transformation|GetActorLocation (Variables|Default|GetGardian%20Plant)))) 0.0)) -1.0)) "1,1,1") "Undefined" 0 0))
    (Default|SetGardianPlant _returnvalue_4 (Variables|Default|GetGardian%20Plant))
    (else
      (Development|PrintString "Error: No Spawn Volumes Provided!" true true "(R=1.000000,G=0.069411,B=0.000000,A=1.000000)"))))

(fn CheckSpawnNewWeed
  (Utilities|FlowControl|Sequence
    (:then_0
      (bind _outactors (Actor|GetAllActorsOfClass "/Game/Blueprints/Enemies/WeedEnemy.WeedEnemy_C"))
      (LocalVariables|SetAll%20Weed%20Plants _outactors))
    (:then_1
      (if (< (Utilities|Array|Length (LocalVariables|GetAll%20Weed%20Plants)) (Variables|Default|GetMax%20Weed%20Count)) ; If we did not reach the max count
        (Utilities|FlowControl|Sequence ; Get available locations
          (:then_0
            (for _array_element (Variables|Default|GetWeed%20Spawn%20Locations) ; Get all
              (Utilities|Array|Add (LocalVariables|GetAvailable%20Locations) (Transformation|GetActorLocation _array_element))))
          (:then_1
            (for (_array_element_2 _array_index) (LocalVariables|GetAvailable%20Locations) ; Substract already used
              (for _array_element_3 (LocalVariables|GetAll%20Weed%20Plants)
                (if (< (Math|Vector|Distance(Vector) (Transformation|GetActorLocation _array_element_3) _array_element_2) 0.1) ; Location too close!
                  (Utilities|Array|RemoveIndex (LocalVariables|GetAvailable%20Locations) _array_index))))
            (LocalVariables|SetNumAvailableLoc (Utilities|Array|Length (LocalVariables|GetAvailable%20Locations))))
          (:then_2
            (if (<= (LocalVariables|GetNumAvailableLoc) 0) ; Return if no available locations
              (return)))
          (:then_3
            (bind _returnvalue (Game|SpawnActorfromClass "/Game/Blueprints/Enemies/WeedEnemy.WeedEnemy_C" (Math|Transform|MakeTransform (Utilities|Array|Get(acopy) (LocalVariables|GetAvailable%20Locations) (Math|Random|RandomIntegerinRange 0 (- (LocalVariables|GetNumAvailableLoc) 1))) "0, 0, 0" "1,1,1") "Undefined" 0 0))
            (Default|SetGardianPlant _returnvalue (Variables|Default|GetGardian%20Plant))))))))

(fn InitializeDefaultsfromDataTable
  (Utilities|FlowControl|Sequence
    (:then_0
      (bind _returnvalue (Utilities|GetDataTableRow "/Game/DataTables/GameplayTuning.GameplayTuning" "AphidSpawnTimer")
        (:then
          (Variables|Default|SetBug%20Spawn%20Timer (.value _returnvalue)))))
    (:then_1
      (bind _returnvalue_2 (Utilities|GetDataTableRow "/Game/DataTables/GameplayTuning.GameplayTuning" "WeedSpawnTimer")
        (:then
          (Variables|Default|SetWeed%20Spawn%20Timer (.value _returnvalue_2)))))
    (:then_2
      (bind _returnvalue_3 (Utilities|GetDataTableRow "/Game/DataTables/GameplayTuning.GameplayTuning" "MaxWeedPlants")
        (:then
          (Variables|Default|SetMax%20Weed%20Count (Math|Float|Truncate (.value _returnvalue_3))))))))