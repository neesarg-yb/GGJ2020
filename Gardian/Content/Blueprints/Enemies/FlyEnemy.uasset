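; Flying bug enemy that cycles through On Ground, Take Off, Shoot and Landing states, and destroys itself on DealDamage.
; Tick runs the state machine, with each state setting a timer on entry to switch to the next, and prints the state for debugging.
; Timer durations come from GameplayTuning data table rows via InitalizeVariablesFromDataTable, which this graph never calls.
; Per-state update functions are empty stubs, and the guardian plant reference is only stored.
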(event Custom|Event%20Tick%20-%20On%20Ground
  (params (Delta%20Seconds :type Float%20%28single-precision%29))
  ;[1 1 1] State: On Ground
  (Utilities|FlowControl|Sequence
    (:then_0
      (if (!= (Variables|Default|GetLastFrameState) (Variables|Default|GetThisFrameState))
        (Utilities|Time|SetTimerbyEvent (delegate Custom|ChangeToTakeOff) (Variables|Default|GetSecondsOnGround))))
    (:then_1
      (CallFunction|UpdateonGround))))

(event Custom|Event%20Tick%20-%20Take%20Off
  (params (Delta%20Seconds :type Float%20%28single-precision%29))
  ;[1 1 1] State: Take Off
  (Utilities|FlowControl|Sequence
    (:then_0
      (if (!= (Variables|Default|GetLastFrameState) (Variables|Default|GetThisFrameState))
        (Utilities|Time|SetTimerbyEvent (delegate Custom|ChangeToShoot) (Variables|Default|GetSecondsFlyingUpOrDown))))
    (:then_1
      (CallFunction|UpdateTakeOff))))

(event Custom|Event%20Tick%20-%20Shoot
  (params (Delta%20Seconds :type Float%20%28single-precision%29))
  ;[1 1 1] State: Shoot
  (Utilities|FlowControl|Sequence
    (:then_0
      (if (!= (Variables|Default|GetLastFrameState) (Variables|Default|GetThisFrameState))
        (Utilities|Time|SetTimerbyEvent (delegate Custom|ChangeToLanding) (Variables|Default|GetSecondsWaitAfterShoot))))
    (:then_1
      (CallFunction|UpdateShoot))))

(event Custom|Event%20Tick%20-%20Landing
  (params (Delta%20Seconds :type Float%20%28single-precision%29))
  ;[1 1 1] State: Landing
  (Utilities|FlowControl|Sequence
    (:then_0
      (if (!= (Variables|Default|GetLastFrameState) (Variables|Default|GetThisFrameState))
        (Utilities|Time|SetTimerbyEvent (delegate Custom|ChangeToOnGound) (Variables|Default|GetSecondsFlyingUpOrDown))))
    (:then_1
      (CallFunction|UpdateLanding))))

(event Custom|ChangeToTakeOff
  ;[1 1 1] State: On Ground
  (Variables|Default|SetThisFrameState "NewEnumerator1"))

(event Custom|ChangeToShoot
  ;[1 1 1] State: Take Off
  (Variables|Default|SetThisFrameState "NewEnumerator2"))

(event Custom|ChangeToLanding
  ;[1 1 1] State: Shoot
  (Variables|Default|SetThisFrameState "NewEnumerator3"))

(event Custom|ChangeToOnGound
  ;[1 1 1] State: Landing
  (Variables|Default|SetThisFrameState "NewEnumerator0"))

(event EventBeginPlay)

(event Collision|EventActorBeginOverlap
  (params (OtherActor :type Actor%20Object%20Reference))
  (|CallParentFunction OtherActor) ; This node is disabled and will not be called.\nDrag off pins to build functionality.
)

(event EventTick
  (params (DeltaSeconds :type Float%20%28single-precision%29))
  (Variables|Default|SetDeltaSeconds DeltaSeconds)
  (CallFunction|DebugPrintCurrentState)
  (Utilities|FlowControl|Sequence
    (:then_0
      (switch Utilities|FlowControl|Switch|SwitchonFlyBugStates (Variables|Default|GetThisFrameState)
        (:NewEnumerator0
          (CallFunction|EventTick-onGround (Variables|Default|GetDeltaSeconds)))
        (:NewEnumerator1
          (CallFunction|EventTick-TakeOff (Variables|Default|GetDeltaSeconds)))
        (:NewEnumerator2
          (CallFunction|EventTick-Shoot (Variables|Default|GetDeltaSeconds)))
        (:NewEnumerator3
          (CallFunction|EventTick-Landing (Variables|Default|GetDeltaSeconds)))))
    (:then_1
      (if (!= (Variables|Default|GetLastFrameState) (Variables|Default|GetThisFrameState)) ; Peek next state
        (Variables|Default|SetSecondsInCurrentState 0.0) ; State just changed?
        (else
          (Variables|Default|SetSecondsInCurrentState (+ (Variables|Default|GetSecondsInCurrentState) (Variables|Default|GetDeltaSeconds))) ; We're in the same state
        )))
    (:then_2
      (Variables|Default|SetLastFrameState (Variables|Default|GetThisFrameState)))))

(fn ConstructionScript
  (|CallParentFunction))

(fn SetGardianPlant
  (params (Plant :type Plant%20Object%20Reference))
  (Variables|Default|SetGardianPlant Plant))

(fn DealDamage
  (|CallParentFunction)
  (Actor|DestroyActor))

(fn UpdateonGround)

(fn UpdateTakeOff)

(fn UpdateShoot)

(fn UpdateLanding)

(fn DebugPrintCurrentState
  (Utilities|FlowControl|Sequence
    (:then_0
      (switch Utilities|FlowControl|Switch|SwitchonFlyBugStates (Variables|Default|GetThisFrameState)
        (:NewEnumerator0
          (LocalVariables|SetStateName "ON GROUND"))
        (:NewEnumerator1
          (LocalVariables|SetStateName "TAKE OFF"))
        (:NewEnumerator2
          (LocalVariables|SetStateName "SHOOT"))
        (:NewEnumerator3
          (LocalVariables|SetStateName "LANDING"))))
    (:then_1
      (Development|PrintString (Utilities|String|Append "\"" (Utilities|GetDisplayName self) "\" in state: " (LocalVariables|GetStateName) " (" (Utilities|String|ToString(Float) (Variables|Default|GetSecondsInCurrentState)) " sec)") true true "(R=1.000000,G=0.785571,B=0.000000,A=1.000000)" 0.0))))

(fn InitalizeVariablesfromDataTable
  (Utilities|FlowControl|Sequence
    (:then_0
      (bind _returnvalue (Utilities|GetDataTableRow "/Game/DataTables/GameplayTuning.GameplayTuning" "FlyBugOnGroundTimer")
        (:then
          (Variables|Default|SetSecondsOnGround (.value _returnvalue)))))
    (:then_1
      (bind _returnvalue_2 (Utilities|GetDataTableRow "/Game/DataTables/GameplayTuning.GameplayTuning" "FlyBugTransitionUpDownTimer")
        (:then
          (Variables|Default|SetSecondsFlyingUpOrDown (.value _returnvalue_2)))))
    (:then_2
      (bind _returnvalue_3 (Utilities|GetDataTableRow "/Game/DataTables/GameplayTuning.GameplayTuning" "FlyBugAfterShootInAirTimer")
        (:then
          (Variables|Default|SetSecondsWaitAfterShoot (.value _returnvalue_3)))))))