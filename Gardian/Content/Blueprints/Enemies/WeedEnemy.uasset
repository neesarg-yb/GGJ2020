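; Weed enemy Blueprint that harms an assigned guardian plant and destroys itself once its inherited DealDamage runs.
; On BeginPlay it reads its attack delay from the GameplayTuning data table and starts a looping timer with that interval.
; The guardian plant is set through SetGardianPlant, and DamageTheGardianPlant shrinks it and prints a debug message.
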(event EventBeginPlay
  (CallFunction|InitializeDefaultsfromDataTable)
  (Utilities|Time|SetTimerbyEvent (EventDispatchers|CreateEvent :!event DamagetheGardianPlant) (Variables|Default|GetAttackPlantAfter?Seconds) true))

(event Collision|EventActorBeginOverlap
  (params (OtherActor :type Actor%20Object%20Reference)))

(event EventTick
  (params (DeltaSeconds :type Float%20%28single-precision%29)))

(fn ConstructionScript
  (Variables|Default|Setprim (Variables|Default|GetStaticMeshWeedPlant))
  (Variables|Default|Setcolor "(R=1.000000,G=1.000000,B=1.000000,A=1.000000)")
  (|CallParentFunction))

(fn DealDamage
  (|CallParentFunction)
  (Actor|DestroyActor))

(fn SetGardianPlant
  (params (Plant :type Plant%20Object%20Reference))
  (Variables|Default|SetGardianPlant Plant))

(fn DamagetheGardianPlant
  (Default|Shrink (Variables|Default|GetGardianPlant) false)
  (Development|PrintString (Utilities|String|Append "Enemy \"" (Utilities|GetDisplayName self) "\" dealt damage to Plant!") true true "(R=1.000000,G=0.034090,B=0.000000,A=1.000000)"))

(fn InitializeDefaultsfromDataTable
  (Utilities|FlowControl|Sequence
    (:then_0
      (bind _returnvalue (Utilities|GetDataTableRow "/Game/DataTables/GameplayTuning.GameplayTuning" "WeedDealDamageToPlantTimer")
        (:then
          (Variables|Default|SetAttackPlantAfter?Seconds (.value _returnvalue)))))))