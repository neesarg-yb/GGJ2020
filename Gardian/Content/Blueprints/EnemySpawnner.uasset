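; Enemy spawner actor that periodically creates AphidEnemy actors inside designated spawn volumes.
; BeginPlay starts a looping timer at the SpawnTimeSeconds interval to drive spawning.
; SpawnNewEnemy derives a random position from SpawnVolume bounds, spawns there and prints a volume name, or an error if none exist.
; The random volume index is evaluated more than once, so the printed name can differ from the volume used.
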(event EventBeginPlay
  (Utilities|Time|SetTimerbyEvent (EventDispatchers|CreateEvent :!event SpawnNewEnemy) (Variables|Default|GetSpawn%20Time%20Seconds) true))

(event Collision|EventActorBeginOverlap
  (params (OtherActor :type Actor%20Object%20Reference)))

(event EventTick
  (params (DeltaSeconds :type Float%20%28single-precision%29)))

(fn ConstructionScript)

(fn SpawnNewEnemy
  (bind _spawn_volume (Variables|Default|GetSpawn%20Volume))
  (bind _spawn_volume_2 (Variables|Default|GetSpawn%20Volume))
  (bind _returnvalue (Utilities|Array|Length _spawn_volume))
  (bind _returnvalue_2 (- _returnvalue 1))
  (bind _returnvalue_3 (Math|Random|RandomIntegerinRange 0 _returnvalue_2))
  (bind _output (Utilities|Array|Get(acopy) _spawn_volume_2 _returnvalue_3))
  (bind (_origin _boxextent) (Collision|GetActorBounds _output false))
  (if (> (Utilities|Array|Length (Variables|Default|GetSpawn%20Volume)) 0)
    (LocalVariables|SetVolume%20Name (Utilities|GetObjectName _output))
    (bind _position_out (CallFunction|GetRandomPositionfromVolume _origin _boxextent))
    (Game|SpawnActorfromClass "/Game/Blueprints/Enemies/AphidEnemy.AphidEnemy_C" (Math|Transform|MakeTransform _position_out "0, 0, 0" "1,1,1") "Undefined" 0 0)
    (Development|PrintString (Utilities|String|Append (Utilities|String|MakeLiteralString "Spawnned an Enemy in \"") (Utilities|String|MakeLiteralString (LocalVariables|GetVolume%20Name)) (Utilities|String|MakeLiteralString "\".")))
    (else
      (Development|PrintString "Error: No Spawn Volumes Provided!" true true "(R=1.000000,G=0.069411,B=0.000000,A=1.000000)"))))