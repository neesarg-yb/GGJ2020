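; MathUtility is a utility Blueprint whose GetRandomPositionFromVolume function returns a random point inside an axis-aligned box.
; It rolls each axis separately between the positive and negative value of an Extents vector, so the extents act as half-sizes.
; The three results form an offset vector that is added to the supplied Center.
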(fn GetRandomPositionfromVolume
  (params (Center :type Vector) (Extents :type Vector))
  (LocalVariables|Setcenter-coord Center)
  (LocalVariables|Setx-coord (.x Extents))
  (LocalVariables|Sety-coord (.y Extents))
  (LocalVariables|Setz-coord (.z Extents))
  (Utilities|FlowControl|Sequence
    (:then_0
      (LocalVariables|Setx-coord_out (Math|Random|RandomFloatinRange (LocalVariables|Getx-coord) (* (LocalVariables|Getx-coord) -1.0))))
    (:then_1
      (LocalVariables|Sety-coord_out (Math|Random|RandomFloatinRange (LocalVariables|Gety-coord) (* (LocalVariables|Gety-coord) -1.0))))
    (:then_2
      (LocalVariables|Setz-coord_out (Math|Random|RandomFloatinRange (LocalVariables|Getz-coord) (* (LocalVariables|Getz-coord) -1.0))))
    (:then_3
      (return (+ (LocalVariables|Getcenter-coord) (Math|Vector|MakeVector (LocalVariables|Getx-coord_out) (LocalVariables|Gety-coord_out) (LocalVariables|Getz-coord_out)))))))