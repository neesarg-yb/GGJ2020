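; GardienCameraActor is a camera actor that applies a procedural, trauma-style screen shake to its camera component.
; AddShake raises a clamped shake amount, which Tick decays linearly over time before calling DoShake.
; DoShake offsets the camera's relative location with time-driven Perlin noise on three random seeds, scaled by that amount.
; The X key triggers a test shake with a debug print.
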(event EventBeginPlay
  (Variables|Default|Setseed1 (Math|Random|RandomFloat))
  (Variables|Default|Setseed2 (Math|Random|RandomFloat))
  (Variables|Default|Setseed3 (Math|Random|RandomFloat))
  (Input|EnableInput (Game|GetPlayerController 0)))

(event Collision|EventActorBeginOverlap
  (params (OtherActor :type Actor%20Object%20Reference)))

(event EventTick
  (params (DeltaSeconds :type Float%20%28single-precision%29))
  ;[1 1 1] Decrement Shake Amount
  (Variables|Default|SetshakeAmount (Math|Float|Clamp(Float) (- (Variables|Default|GetshakeAmount) DeltaSeconds) 0.0 1.0))
  (CallFunction|DoShake))

(event Input|KeyboardEvents|X
  (params (Key :type Key%20Structure :default "None"))
  (:Pressed
    (CallFunction|AddShake 0.5)
    (Development|PrintString "SHAKE" true true "(R=0.189217,G=1.000000,B=0.050196,A=1.000000)")))

(fn ConstructionScript)

(fn AddShake
  (params (shake :type Float%20%28single-precision%29))
  (Variables|Default|SetshakeAmount (Math|Float|Clamp(Float) (+ shake (Variables|Default|GetshakeAmount)))))

(fn DoShake
  (bind _returnvalue (Utilities|Time|GetGameTimeinSeconds))
  (bind _returnvalue_2 (* _returnvalue 25.0))
  (Transformation|SetRelativeLocation (Variables|CameraActor|GetCameraComponent) (* (* (Math|Vector|MakeVector (Class|KismetMathLibrary|PerlinNoise1D (+ (Variables|Default|Getseed1) _returnvalue_2)) (Class|KismetMathLibrary|PerlinNoise1D (+ (Variables|Default|Getseed2) _returnvalue_2)) (Class|KismetMathLibrary|PerlinNoise1D (+ (Variables|Default|Getseed3) _returnvalue_2))) (Variables|Default|GetshakeAmount)) 2e+01) false false))