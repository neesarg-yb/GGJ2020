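; GardienPawn is a pawn that steers relative to the first CameraActor found at BeginPlay.
; Each Tick combines the camera's yaw with the angle of the MoveForward/MoveRight input to set the pawn's rotation.
; It then moves a fixed step along that facing, without sweep or delta time.
; The movement check tests the camera's horizontal forward length rather than input, so it moves unless the camera is near vertical.
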(event EventBeginPlay
  (bind _outactors (Actor|GetAllActorsOfClass "/Script/Engine.CameraActor"))
  (Variables|Default|Setcamera (Utilities|Array|Get(acopy) _outactors)))

(event Collision|EventActorBeginOverlap
  (params (OtherActor :type Actor%20Object%20Reference)))

(event EventTick
  (params (DeltaSeconds :type Float%20%28single-precision%29))
  (bind _camera (Variables|Default|Getcamera))
  (bind _returnvalue (Transformation|GetActorForwardVector _camera))
  (bind (_x _y) (Math|Vector|BreakVector _returnvalue))
  (Transformation|SetActorRotation (Math|Rotator|CombineRotators (Math|Rotator|MakeRotator 0.0 0.0 (Class|KismetMathLibrary|DegAtan2 _y _x)) (Math|Vector|RotatorfromAxisandAngle "0,0.000000,1.000000" (Class|KismetMathLibrary|DegAtan2 (Input|AxisValues|GetMoveRight) (Input|AxisValues|GetMoveForward)))))
  (if (> (Math|Vector|VectorLength (Math|Vector|MakeVector _x _y 0.0)) 0.1)
    (Transformation|AddActorWorldOffset (* (Math|Vector|GetForwardVector (Transformation|GetActorRotation)) 1e+01))))

(fn ConstructionScript)