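; Player pawn for a gardening game with combat: it runs around, attacks Enemy actors and waters Plant actors to grow them.
; Tick turns input camera-relative using the GardienCameraActor found at BeginPlay, then offsets the pawn without sweep, with foot particles and sine squash-bounce.
; Attack and Water share a forward sphere-overlap probe.
; Attacks play hit-or-miss audio and shake the camera on hits; watering still draws a debug sphere.
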(event EventBeginPlay
  (bind _outactors (Actor|GetAllActorsOfClass "/Game/Blueprints/GardienCameraActor.GardienCameraActor_C"))
  (Variables|Default|Setcamera (Utilities|Array|Get(acopy) _outactors)))

(event Collision|EventActorBeginOverlap
  (params (OtherActor :type Actor%20Object%20Reference)))

(event EventTick
  (params (DeltaSeconds :type Float%20%28single-precision%29))
  (CallFunction|DoMovement DeltaSeconds))

(event Input|ActionEvents|InputActionAttack
  (params (Key :type Key%20Structure))
  (:Pressed
    (CallFunction|HandleAttack)))

(event Input|ActionEvents|InputActionWater
  (params (Key :type Key%20Structure))
  (:Pressed
    (CallFunction|HandleWatering)))

(fn ConstructionScript)

(fn DoMovement
  (params (deltaTime :type Float%20%28single-precision%29))
  (bind _returnvalue (Utilities|Time|GetGameTimeinSeconds))
  (bind _returnvalue_2 (Input|AxisValues|GetMoveForward))
  (bind _returnvalue_3 (Input|AxisValues|GetMoveRight))
  (bind _camera (Variables|Default|Getcamera))
  (bind _returnvalue_4 (Transformation|GetActorForwardVector _camera))
  (bind _returnvalue_5 (* _returnvalue 25.0))
  (bind _returnvalue_6 (Math|Trig|Sin(Radians) _returnvalue_5))
  (bind (_x _y) (Math|Vector|BreakVector _returnvalue_4))
  (if (> (Math|Vector|VectorLength (Math|Vector|MakeVector _returnvalue_2 _returnvalue_3 0.0)) 0.1)
    (Transformation|SetActorRotation (Math|Rotator|Lerp(Rotator) (Transformation|GetActorRotation) (Math|Rotator|CombineRotators (Math|Rotator|MakeRotator 0.0 0.0 (Class|KismetMathLibrary|DegAtan2 _y _x)) (Math|Vector|RotatorfromAxisandAngle "0,0.000000,1.000000" (Class|KismetMathLibrary|DegAtan2 _returnvalue_3 _returnvalue_2))) (* deltaTime 3e+01) true) true)
    (Transformation|AddActorWorldOffset (* (Math|Vector|GetForwardVector (Transformation|GetActorRotation)) (Variables|Default|GetrunSpeed)))
    (Effects|Components|ParticleSystem|SetEmitterEnable (Variables|Default|GetfeetParticles) "Particle Emitter" true)
    ;[1 1 1] Bounce
    (Transformation|SetRelativeScale3D (Variables|Default|GetStaticMesh) (Math|Vector|MakeVector 0.75 (+ (* _returnvalue_6 0.08) 0.75) (+ (* _returnvalue_6 -0.08) 0.75)))
    (Variables|Default|SetcachedRotation (Transformation|GetActorRotation))
    (else
      (Effects|Components|ParticleSystem|SetEmitterEnable (Variables|Default|GetfeetParticles) "Particle Emitter" false)
      (Transformation|SetActorRotation (Variables|Default|GetcachedRotation))
      (Transformation|SetRelativeScale3D (Variables|Default|GetStaticMesh) "0.750000,0.750000,0.750000"))))

(fn HandleAttack
  (bind _playerattackaudio (Variables|Default|GetPlayerAttackAudio))
  (bind _outactors (Collision|SphereOverlapActors (+ (Transformation|GetActorLocation) (* (Transformation|GetActorForwardVector) 5e+01)) (Variables|Default|GetattackProbeRadius) (Utilities|Array|MakeArray "ObjectTypeQuery4") "/Game/Blueprints/Enemies/Enemy.Enemy_C"))
  (for _array_element _outactors
    (bind _asenemy (Utilities|Casting|CastToEnemy _array_element))
    (Default|DealDamage _asenemy))
  (Effects|Components|ParticleSystem|SetBoolParameter _playerattackaudio "success" (> (Utilities|Array|Length _outactors) 0))
  (Audio|Components|Audio|Play _playerattackaudio 0.0)
  (if (> (Utilities|Array|Length _outactors) 0)
    (Default|AddShake (Variables|Default|Getcamera) 0.3)))

(fn HandleWatering
  (bind _returnvalue (Transformation|GetActorLocation))
  (bind _returnvalue_2 (Transformation|GetActorForwardVector))
  (bind _attackproberadius (Variables|Default|GetattackProbeRadius))
  (bind _returnvalue_3 (* _returnvalue_2 5e+01))
  (bind _returnvalue_4 (+ _returnvalue _returnvalue_3))
  (Rendering|Debug|DrawDebugSphere _returnvalue_4 _attackproberadius 12 "(R=1.000000,G=0.024480,B=0.000000,A=1.000000)" 0.3 1.0)
  (bind _outactors (Collision|SphereOverlapActors _returnvalue_4 _attackproberadius (Utilities|Array|MakeArray "ObjectTypeQuery2") "/Game/Blueprints/Plant.Plant_C"))
  (for _array_element _outactors
    (bind _asplant (Utilities|Casting|CastToPlant _array_element))
    (Default|Grow _asplant)))